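; BP_Test_Tile is a grid tile actor that holds soil data and a grid position and can host one placed object.
; Add and remove functions snap an actor to the tile with a yaw offset or destroy it, tracking occupancy.
; OpenMenu creates a BPW_TileUI widget filled with the tile's data, and SetTileColor drives hover highlighting through material parameters.
; Hover, click and selection events are empty stubs, so nothing here calls these functions.
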(event EventBeginPlay)

(event Collision|EventActorBeginOverlap
  (params (OtherActor :type Actor%20Object%20Reference)))

(event EventTick
  (params (DeltaSeconds :type Float%20%28single-precision%29)))

(event EventHovered)

(event EventSelectedTick)

(event EventClicked)

(event EventClickedOff
  (params (Actor :type Actor%20Object%20Reference)))

(fn ConstructionScript)

(fn OpenMenu
  (Utilities|IsValid (Variables|Default|GetTileMenu)
    (:Is%20Not%20Valid
      (bind _returnvalue (UserInterface|CreateWidget "/Game/Blueprints/BPW_TileUI.BPW_TileUI_C" (Game|GetPlayerController 0)))
      (bind _output_get (Variables|Default|SetTileMenu _returnvalue))
      (UserInterface|Viewport|AddtoViewport _output_get 0)
      (CallFunction|UpdateMenuInfo))))

(fn CloseMenu
  (Widget|RemovefromParent (Variables|Default|GetTileMenu))
  (Variables|Default|SetTileMenu 0))

(fn UpdateMenuInfo
  (Default|UpdateMenuInfo (Variables|Default|GetTileMenu) 0 (Variables|Default|GetSoilData) (Variables|Default|GetGridPosition) (Variables|Default|GetOccupiedObj)))

(fn RemoveObjectfromTile
  (if (Variables|Default|GetIsOccupied)
    (Actor|DestroyActor (Variables|Default|GetOccupiedObj))
    (Variables|Default|SetOccupiedObj 0)
    (Variables|Default|SetIsOccupied false)))

(fn AddObjecttoTile
  (params (Actor :type Item%20Base%20Object%20Reference) (RotationOffset :type Integer))
  (Utilities|IsValid (Variables|Default|GetOccupiedObj)
    (:Is%20Valid
      (Development|PrintString "Tile Occupied")
      (return false))
    (:Is%20Not%20Valid
      (bind _output_get (Variables|Default|SetOccupiedObj Actor))
      (Transformation|SetActorLocationAndRotation _output_get (Transformation|GetActorLocation) (Math|Rotator|MakeRotator 0.0 0.0 (Math|Conversions|ToFloat(Integer) RotationOffset)))
      (Variables|Default|SetIsOccupied true)
      (return true))))

(fn SetTileColor
  (params (Highlighted :type Boolean) (Color :type Vector))
  (bind _staticmesh (Variables|Default|GetStaticMesh))
  (Rendering|Material|SetScalarParameterValueonMaterials _staticmesh "IsHovered" (Math|Conversions|ToFloat(Boolean) Highlighted))
  (Rendering|Material|SetVectorParameterValueonMaterials _staticmesh "HoverColor" Color))