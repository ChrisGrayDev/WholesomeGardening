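; BP_ProgressBar is a temporary world-space timer bar actor that shows progress through a widget component and removes itself when done.
; StartTimer stores the duration, starts progress on the WBP_Timer widget and sets a timer that calls StopTimer to destroy the actor.
; On Tick, the widget component rotates to face the player camera as a billboard.
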(event EventBeginPlay)

(event Collision|EventActorBeginOverlap
  (params (OtherActor :type Actor%20Object%20Reference)))

(event EventTick
  (params (DeltaSeconds :type Float%20%28single-precision%29))
  (bind _widget (Variables|Default|GetWidget))
  (Transformation|SetWorldRotation _widget (Math|Rotator|FindLookatRotation (Transformation|GetWorldLocation _widget) (Transformation|GetActorLocation (Game|GetPlayerCameraManager 0))) false false))

(fn ConstructionScript)

(fn StartTimer
  (params (MaxTime :type Float%20%28single-precision%29))
  (bind _output_get (Variables|Default|SetMaxTime MaxTime))
  (bind _aswbp_timer (Utilities|Casting|CastToWBP_Timer (UserInterface|GetWidget (Variables|Default|GetWidget))))
  (Default|StartProgress _aswbp_timer _output_get)
  (Utilities|Time|SetTimerbyFunctionName self "StopTimer" _output_get))

(fn StopTimer
  (Actor|DestroyActor))