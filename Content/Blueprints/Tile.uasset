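; Grid tile actor that holds a soil type, position, sunlight and one placeable, such as a plant.
; Construction stores a dynamic material instance and picks a random soil type.
; PlacePlant removes the existing placeable or spawns a Plant through PlaceActor, which assigns it and enables growth.
; A TileUI widget opened per tile shows these details and is refreshed whenever the placeable changes.
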(event EventBeginPlay)

(event Collision|EventActorBeginOverlap
  (params (OtherActor :type Actor%20Object%20Reference)))

(event EventTick
  (params (DeltaSeconds :type Float%20%28single-precision%29)))

(fn ConstructionScript
  (bind _returnvalue (Rendering|Material|CreateDynamicMaterialInstance (Variables|Debug|GetStaticMeshComponent) 0 0 "None" :!class /Script/Engine.PrimitiveComponent))
  (Variables|Default|SetDynamicMaterial _returnvalue)
  (Variables|Default|SetSoil (Utilities|Enum|ByteToEnumSoilType (Math|Conversions|ToByte(Integer) (Math|Random|RandomIntegerinRange 0 5)))))

(fn OpenMenu
  (bind _returnvalue (UserInterface|CreateWidget "/Game/Blueprints/TileUI.TileUI_C" (Game|GetPlayerController 0)))
  (bind _output_get (Variables|Default|SetTileMenu _returnvalue))
  (UserInterface|Viewport|AddtoViewport _output_get 0)
  (CallFunction|UpdateMenuInfo))

(fn CloseMenu
  (Widget|RemovefromParent (Variables|Default|GetTileMenu)))

(fn PlacePlant
  (if (Utilities|IsValid (Variables|Default|GetPlaceable))
    (Actor|DestroyActor (Variables|Default|GetPlaceable))
    (Variables|Default|SetPlaceable 0)
    (CallFunction|UpdateMenuInfo)
    (Development|PrintString "cheese")
    (else
      (bind _output_get (Variables|Default|SetStartingTransformPlant (Math|Transform|MakeTransform (Transformation|GetActorLocation) "0, 0, 0" "1,1,1")))
      (bind _returnvalue (Game|SpawnActorfromClass "/Game/Blueprints/Plant.Plant_C" _output_get "Undefined" self 0))
      (CallFunction|PlaceActor _returnvalue))))

(fn PlaceActor
  (params (Placeable :type Placeable%20Base%20Object%20Reference))
  (if (Utilities|IsValid (Variables|Default|GetPlaceable))
    (Actor|DestroyActor (Variables|Default|GetPlaceable))
    (Variables|Default|SetPlaceable 0))
  (bind _output_get (Variables|Default|SetPlaceable Placeable))
  (bind _asplant (Utilities|Casting|CastToPlant _output_get)
    (:then
      (Variables|/Game/Blueprints/Plant.Plant_C|SetEnabledGrowth _asplant true))
    (:CastFailed
      _))
  (CallFunction|UpdateMenuInfo)
  (Development|PrintString "Hello"))

(fn UpdateMenuInfo
  (bind _position (Variables|Default|GetPosition))
  (bind _tilemenu (Variables|Default|GetTileMenu))
  (if (Utilities|IsValid _tilemenu)
    (Variables|/Game/Blueprints/TileUI.TileUI_C|SetSoilTypeText _tilemenu (Utilities|String|Append "Soil Type: " (Utilities|String|EnumtoString (Variables|Default|GetSoil))))
    (Variables|/Game/Blueprints/TileUI.TileUI_C|SetTilePositionText _tilemenu (Utilities|String|Append "Position: (" (Utilities|String|ToString(Integer) (Math|Float|Truncate (.x _position))) "," (Utilities|String|ToString(Integer) (Math|Float|Truncate (.y _position))) ")"))
    (Variables|/Game/Blueprints/TileUI.TileUI_C|SetSunlightText _tilemenu (Utilities|String|Append "Sunlight: " (Utilities|String|ToString(Boolean) (Variables|Default|GetSunlight))))
    (Variables|/Game/Blueprints/TileUI.TileUI_C|SetTileRef _tilemenu self)
    (Variables|/Game/Blueprints/TileUI.TileUI_C|SetPlaceableOnTile _tilemenu (Utilities|GetDisplayName (Variables|Default|GetPlaceable)))))