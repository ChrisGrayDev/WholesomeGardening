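; Grid-based building system that places data-driven plants on Tile actors under the mouse cursor.
; While building, each tick traces from the cursor to find the hovered tile and moves a hologram preview there, coloured by whether the tile is free.
; Rotation input snaps in 90-degree steps.
; SpawnObject spawns a BP_Plant initialised from its PlantTable row, then registers it with the tile or destroys it if occupied.
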(event Custom|OnRotateClockWise
  (CallFunction|RotateOffset true))

(event Custom|OnRotateAntiClockwise
  (CallFunction|RotateOffset false))

(event EventBeginPlay)

(event EventTick
  (params (DeltaSeconds :type Float%20%28single-precision%29))
  (Utilities|FlowControl|Sequence
    (:then_0
      (CallFunction|GetHoveredTile))
    (:then_1
      (CallFunction|SpawnHologram))
    (:then_2
      (CallFunction|SetActortoGridLocation (Variables|Default|GetPreviewObj)))))

(fn SpawnObject
  (bind _hoveredtile (Variables|Default|GetHoveredTile))
  (bind _previewobj (Variables|Default|GetPreviewObj))
  (if (Utilities|IsValid (Variables|Default|GetHoveredTile))
    (if (Variables|Default|GetCanBuildHere)
      (if (Variables|Default|GetIsBuilding)
        (bind _out (CallFunction|SpawnPlantfromName (Utilities|String|StringToName (.name (Utilities|Struct|BreakItemData (Variables|Default|GetActiveItem))))))
        (Transformation|SetActorLocationAndRotation _out (.location (Variables|Default|GetTilePlaceLocation)) (Math|Rotator|MakeRotator 0.0 0.0 (Math|Conversions|ToFloat(Integer) (Variables|Default|GetRotationSnapOffset))))
        (Variables|Default|SetIsBuilding false)
        (if (Utilities|IsValid _previewobj)
          (Actor|DestroyActor _previewobj)
          (if (Utilities|IsValid (Variables|Default|GetHoveredTile))
            (if (Variables|/Game/Blueprints/Tile.Tile_C|GetIsOccupied _hoveredtile)
              (Actor|DestroyActor _out)
              (else
                (Default|SetOwningObject _hoveredtile)))
            (else
              (Actor|DestroyActor _out)))))
      (else
        (Development|PrintString "Cannot build here")))))

(fn ToggleIsBuilding
  (bind _previewobj (Variables|Default|GetPreviewObj))
  (if (Variables|Default|GetIsBuilding)
    (Variables|Default|SetIsBuilding false)
    (if (Utilities|IsValid _previewobj)
      (Actor|DestroyActor _previewobj))
    (else
      (Variables|Default|SetIsBuilding true))))

(fn RotateOffset
  (params (Clockwise :type Boolean))
  (if Clockwise
    (bind _output_get (Variables|Default|SetRotationSnapOffset (+ (Variables|Default|GetRotationSnapOffset) 90)))
    (else
      (Variables|Default|SetRotationSnapOffset (+ (Variables|Default|GetRotationSnapOffset) -90))))
  (if (>= _output_get 360)
    (Variables|Default|SetRotationSnapOffset (+ (Variables|Default|GetRotationSnapOffset) -360))
    (elif (not (>= (Variables|Default|GetRotationSnapOffset) 0))
      (Variables|Default|SetRotationSnapOffset (+ (Variables|Default|GetRotationSnapOffset) 360)))))

(fn SpawnPlantfromName
  (params (PlantName :type Name))
  (bind _returnvalue (Game|SpawnActorfromClass "/Game/Blueprints/BP_Plant.BP_Plant_C" (Variables|Default|GetZeroLocation) "Undefined" 0 0))
  (bind _returnvalue_2 (Utilities|GetDataTableRow (Variables|Default|GetPlantTable) PlantName)
    (:then
      (Class|Plant|InitPlant _returnvalue _returnvalue_2)
      (return _returnvalue))))

(fn GetHoveredTile
  (bind _returnvalue (Game|GetPlayerController 0))
  (bind _previewobj (Variables|Default|GetPreviewObj))
  (bind (_worldlocation _worlddirection) (Game|Player|ConvertMouseLocationToWorldSpace _returnvalue))
  ;[1 1 1] Line Trace and Get Tile Location
  (if (Variables|Default|GetIsBuilding)
    (bind _outhit (Collision|LineTraceByChannel _worldlocation (+ (* _worlddirection 4e+03) _worldlocation) "TraceTypeQuery1" false 0 "None"))
    (Variables|Default|SetCursorTransform (Math|Conversions|ToTransform(Vector) (.Location (Collision|BreakHitResult _outhit))))
    (bind _astile (Utilities|Casting|CastToTile (.HitActor (Collision|BreakHitResult _outhit)))
      (:then
        (bind _output_get (Variables|Default|SetHoveredTile _astile))
        (Variables|Default|SetTilePlaceLocation (Transformation|GetActorTransform _output_get))
        (if (Utilities|IsValid _previewobj)
          (if (Variables|/Game/Blueprints/Tile.Tile_C|GetIsOccupied _output_get)
            (Default|SetHologramColour _previewobj false)
            (Variables|Default|SetCanBuildHere false)
            (else
              (Default|SetHologramColour _previewobj true)
              (Variables|Default|SetCanBuildHere true)))))
      (:CastFailed
        (Variables|Default|SetTilePlaceLocation "")
        (Variables|Default|SetHoveredTile 0)))))

(fn SetActortoGridLocation
  (params (Actor :type Actor%20Object%20Reference))
  (if (Utilities|IsValid Actor)
    (if (Utilities|IsCurrentTileLocationZero)
      (CallFunction|DestroyActor (Variables|Default|GetPreviewObj))
      (Variables|Default|SetTilePlaceLocation "")
      (else
        (Transformation|SetActorLocationAndRotation Actor (.location (Variables|Default|GetTilePlaceLocation)) (Math|Rotator|MakeRotator 0.0 0.0 (Math|Conversions|ToFloat(Integer) (Variables|Default|GetRotationSnapOffset))))))))

(fn DestroyActor
  (params (Actor :type Actor%20Object%20Reference))
  (if (Utilities|IsValid Actor)
    (Actor|DestroyActor Actor)
    (Variables|Default|SetTilePlaceLocation "")))

(fn SpawnHologram
  ;[1 1 1] Spawn Hologram Plant
  (if (Variables|Default|GetIsBuilding)
    (if (and (Utilities|IsValid (Variables|Default|GetHoveredTile)) (not (Utilities|IsValid (Variables|Default|GetPreviewObj))))
      (Development|PrintString "Plant spawned")
      (bind _returnvalue (Game|SpawnActorfromClass "/Game/Blueprints/BP_PreviewObj.BP_PreviewObj_C" (Variables|Default|GetTilePlaceLocation) "Undefined" 0 0))
      (bind _output_get (Variables|Default|SetPreviewObj _returnvalue))
      (Default|SetHologramColour _output_get false))
    (else
      (CallFunction|DestroyActor (Variables|Default|GetPreviewObj)))))