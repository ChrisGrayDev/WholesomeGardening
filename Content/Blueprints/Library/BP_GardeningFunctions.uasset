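; Blueprint function library of shared helpers for the gardening gameplay.
; Hover functions set IsHovered and CantUse scalars on slot 0 dynamic materials of static or skeletal meshes for valid or invalid highlights, and tile visibility sets Alpha across BP_TileManager's tiles.
; Other helpers trace under the mouse cursor on the Visibility channel, test actor classes and play particle bursts with sound.
; Inventory helpers query or consume items through BP_PlayerControl, refreshing its UI on removal.
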(fn HoverStaticObj
  (params (StaticMesh :type Static%20Mesh%20Component%20Object%20Reference) (Green :type Boolean))
  (Utilities|IsValid StaticMesh
    (:Is%20Valid
      (bind _asmaterial_instance_dynamic (Utilities|Casting|CastToMaterialInstanceDynamic (Rendering|Material|GetMaterial StaticMesh 0))
        (:then
          (if Green
            (LocalVariables|SetGreenVal 1.0)
            (LocalVariables|SetRedVal 0.0)
            (else
              (LocalVariables|SetGreenVal 0.0)
              (LocalVariables|SetRedVal 1.0)))
          (Rendering|Material|SetScalarParameterValue _asmaterial_instance_dynamic "IsHovered" (LocalVariables|GetGreenVal) :!class /Script/Engine.MaterialInstanceDynamic)
          (Rendering|Material|SetScalarParameterValue _asmaterial_instance_dynamic "CantUse" (LocalVariables|GetRedVal) :!class /Script/Engine.MaterialInstanceDynamic))
        (:CastFailed
          (Development|PrintString 0 "dynamic material cast failed" true true "(R=0.000000,G=0.660000,B=1.000000,A=1.000000)" (Utilities|Time|GetWorldDeltaSeconds)))))))

(fn UnHoverStaticObj
  (params (StaticMesh :type Static%20Mesh%20Component%20Object%20Reference))
  (bind _asmaterial_instance_dynamic (Utilities|Casting|CastToMaterialInstanceDynamic (Rendering|Material|GetMaterial StaticMesh 0)))
  (Rendering|Material|SetScalarParameterValue _asmaterial_instance_dynamic "IsHovered" 0.0 :!class /Script/Engine.MaterialInstanceDynamic)
  (Rendering|Material|SetScalarParameterValue _asmaterial_instance_dynamic "CantUse" 0.0 :!class /Script/Engine.MaterialInstanceDynamic))

(fn HoverSkeletalObj
  (params (SkeletalMesh :type Skeletal%20Mesh%20Component%20Object%20Reference) (Green :type Boolean))
  (bind _asmaterial_instance_dynamic (Utilities|Casting|CastToMaterialInstanceDynamic (Rendering|Material|GetMaterial SkeletalMesh 0)))
  (if Green
    (LocalVariables|SetGreenVal 1.0)
    (LocalVariables|SetRedVal 0.0)
    (else
      (LocalVariables|SetGreenVal 0.0)
      (LocalVariables|SetRedVal 1.0)))
  (Rendering|Material|SetScalarParameterValue _asmaterial_instance_dynamic "IsHovered" (LocalVariables|GetGreenVal) :!class /Script/Engine.MaterialInstanceDynamic)
  (Rendering|Material|SetScalarParameterValue _asmaterial_instance_dynamic "CantUse" (LocalVariables|GetRedVal) :!class /Script/Engine.MaterialInstanceDynamic))

(fn UnHoverSkeletalObj
  (params (SkeletalMesh :type Skeletal%20Mesh%20Component%20Object%20Reference))
  (bind _asmaterial_instance_dynamic (Utilities|Casting|CastToMaterialInstanceDynamic (Rendering|Material|GetMaterial SkeletalMesh 0)))
  (Rendering|Material|SetScalarParameterValue _asmaterial_instance_dynamic "IsHovered" 0.0 :!class /Script/Engine.MaterialInstanceDynamic)
  (Rendering|Material|SetScalarParameterValue _asmaterial_instance_dynamic "CantUse" 0.0 :!class /Script/Engine.MaterialInstanceDynamic))

(fn IsClassOfType
  (params (Actor :type Actor%20Object%20Reference) (Class :type Actor%20Class%20Reference))
  (return (Utilities|ClassIsChildOf (Utilities|GetClass Actor) Class)))

(fn RaycastActor
  (bind _returnvalue (Game|GetPlayerController 0))
  (bind (_worldlocation _worlddirection) (Game|Player|ConvertMouseLocationToWorldSpace _returnvalue))
  (bind _outhit (Collision|LineTraceByChannel 0 _worldlocation (+ (* _worlddirection 5e+03) _worldlocation) "TraceTypeQuery1" true 0 "None"))
  (return (.HitActor (Collision|BreakHitResult _outhit)) (.Location (Collision|BreakHitResult _outhit))))

(fn PlaySmokeBurst
  (params (Particles :type Actor%20Component%20Object%20Reference))
  (Components|Activation|Activate Particles true)
  (Audio|PlaySound2D 0 "/Game/Sounds/SFX/SC_SmokeBells.SC_SmokeBells" 1.0 1.0 0.0 0 0))

(fn ToggleTileVisibility
  (params (On :type Boolean))
  (bind _returnvalue (Actor|GetActorOfClass 0 "/Game/Blueprints/BP_TileManager.BP_TileManager_C"))
  (if On
    (for _array_element (Variables|/Game/Blueprints/BP_TileManager.BP_TileManager_C|GetTiles _returnvalue)
      (bind _asmaterial_instance_dynamic (Utilities|Casting|CastToMaterialInstanceDynamic (Rendering|Material|GetMaterial (Variables|/Game/Blueprints/BP_Tile.BP_Tile_C|GetStaticMesh _array_element) 0)))
      (Rendering|Material|SetScalarParameterValue _asmaterial_instance_dynamic "Alpha" 0.5 :!class /Script/Engine.MaterialInstanceDynamic))
    (else
      (for _array_element_2 (Variables|/Game/Blueprints/BP_TileManager.BP_TileManager_C|GetTiles _returnvalue)
        (bind _asmaterial_instance_dynamic_2 (Utilities|Casting|CastToMaterialInstanceDynamic (Rendering|Material|GetMaterial (Variables|/Game/Blueprints/BP_Tile.BP_Tile_C|GetStaticMesh _array_element_2) 0)))
        (Rendering|Material|SetScalarParameterValue _asmaterial_instance_dynamic_2 "Alpha" 0.0 :!class /Script/Engine.MaterialInstanceDynamic)))))

(fn PlayPerfectBurst
  (params (Smoke :type Actor%20Component%20Object%20Reference) (Sparks :type Actor%20Component%20Object%20Reference))
  (Components|Activation|Activate Smoke true)
  (Components|Activation|Activate Sparks true)
  (Audio|PlaySound2D 0 "/Game/Sounds/SFX/SC_SmokeBells.SC_SmokeBells" 1.0 1.0 0.0 0 0))

(fn HasIteminInventory
  (params (ItemName :type String))
  (bind _asbp_player_control (Utilities|Casting|CastToBP_PlayerControl (Game|Player|GetPlayerPawn 0))
    (:then
      (bind (_out_id _returnvalue) (Class|InventoryCatalogue|ContainsItem (Variables|/Game/Blueprints/BP_PlayerControl.BP_PlayerControl_C|GetInventoryCatalogue _asbp_player_control) ItemName))
      (LocalVariables|SetLocalHasItem _returnvalue))
    (:CastFailed
      _))
  (return (LocalVariables|GetLocalHasItem) _out_id))

(fn RemoveItem
  (params (ItemID :type Integer))
  (bind _asbp_player_control (Utilities|Casting|CastToBP_PlayerControl (Game|Player|GetPlayerPawn 0)))
  (Class|InventoryCatalogue|RemoveItem (Variables|/Game/Blueprints/BP_PlayerControl.BP_PlayerControl_C|GetInventoryCatalogue _asbp_player_control) ItemID 1)
  (Default|RefreshUsedItem (Variables|/Game/Blueprints/BP_PlayerControl.BP_PlayerControl_C|GetInventoryUI _asbp_player_control) ItemID))