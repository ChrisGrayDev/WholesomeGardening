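; Builder is an actor Blueprint that manages opening and closing the building UI menu.
; OpenMenu opens BuildingUI through MenuManager and stores the result in Menu, which CloseMenu passes back to MenuManager to close.
; ToggleMenu is unfinished, checking Menu validity without acting on it, and the event graph and construction script are empty.
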(event EventBeginPlay)

(event Collision|EventActorBeginOverlap
  (params (OtherActor :type Actor%20Object%20Reference)))

(event EventTick
  (params (DeltaSeconds :type Float%20%28single-precision%29)))

(fn ConstructionScript)

(fn OpenMenu
  (bind _widgetobject (Default|OpenMenu (Variables|Default|GetMenuManager) "/Game/Blueprints/BuildingUI.BuildingUI_C"))
  (Variables|Default|SetMenu _widgetobject))

(fn CloseMenu
  (Default|CloseMenu (Variables|Default|GetMenuManager) (Variables|Default|GetMenu)))

(fn ToggleMenu
  (if (Utilities|IsValid (Variables|Default|GetMenu))
    _))