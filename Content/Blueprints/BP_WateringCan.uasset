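; Watering can actor that the player selects by clicking, then clicks off onto a tile to water the plant occupying it.
; Hover and click events drive skeletal mesh highlighting, selection state and pickup/drop sounds.
; If charges remain and the refilling/extracting check passes, it teleports beside the plant, targets it and extracts one charge.
; StartWatering and StopWatering toggle the Water effect, which is attached to the mesh's Nozzle socket.
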(event EventBeginPlay
  (Transformation|AttachComponentToComponent (Variables|Default|GetWater) (Variables|Character|GetMesh) "Nozzle" "KeepRelative" "KeepRelative" "KeepWorld" true))

(event Collision|EventActorBeginOverlap
  (params (OtherActor :type Actor%20Object%20Reference)))

(event EventHovered
  (if (Variables|Default|GetIsSelected)
    (CallFunction|HoverSkeletalObj (Variables|Character|GetMesh) false)
    (else
      (CallFunction|HoverSkeletalObj (Variables|Character|GetMesh) true))))

(event EventClicked
  (Variables|Default|SetIsSelected true)
  (Audio|PlaySound2D "/Game/Sounds/SFX/SC_WateringCanPickup.SC_WateringCanPickup" 1.0 1.0 0.0 0 0))

(event EventClickedOff
  (params (Actor :type Actor%20Object%20Reference))
  (Audio|PlaySound2D "/Game/Sounds/SFX/SC_WateringCanDrop.SC_WateringCanDrop" 1.0 1.0 0.0 0 0)
  (CallFunction|UnHoverSkeletalObj (Variables|Character|GetMesh))
  (Variables|Default|SetIsSelected false)
  (Utilities|IsValid Actor
    (:Is%20Valid
      (bind _asbp_tile (Utilities|Casting|CastToBP_Tile Actor))
      (bind _asplant (Utilities|Casting|CastToPlant (Variables|/Game/Blueprints/BP_Tile.BP_Tile_C|GetOccupiedObj _asbp_tile)))
      (CallFunction|WaterPlant _asplant))))

(event EventUnhovered
  (CallFunction|UnHoverSkeletalObj (Variables|Character|GetMesh)))

(fn ConstructionScript
  (bind _returnvalue (Rendering|Material|CreateDynamicMaterialInstance "/Game/Models/WateringCan/m_WateringCan.m_WateringCan" "None" "None" :!class /Script/Engine.KismetMaterialLibrary))
  (Rendering|Material|SetMaterial (Variables|Character|GetMesh) 0 _returnvalue))

(fn StartWatering
  (Components|Activation|Activate (Variables|Default|GetWater) false)
  (Audio|PlaySound2D 0 1.0 1.0 0.0 0 0))

(fn StopWatering
  (Components|Activation|Deactivate (Variables|Default|GetWater)))

(fn WaterPlant
  (params (Plant :type Plant%20Object%20Reference))
  (Utilities|IsValid Plant
    (:Is%20Valid
      (bind _returnvalue (Class|WaterExtractable|IsEmpty))
      (if (not _returnvalue)
        (if (not (and (Variables|Default|Getis_refilling) (Variables|Default|Getis_extracting)))
          (Class|WaterExtractable|TeleporttoPoint (+ (Transformation|GetActorLocation Plant) "80.000000,0.000000, 0"))
          (Class|WaterContainer|SetTargetPlant Plant)
          (Class|WaterExtractable|ExtractOneCharge))))))