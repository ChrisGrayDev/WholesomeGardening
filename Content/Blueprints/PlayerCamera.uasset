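; Player camera pawn for a tile-based game that moves, rotates, zooms via spring arm, and picks tiles with the mouse.
; Tick traces from the cursor to track the hovered tile and tints tile dynamic materials for hover and selection, printing the selection's name.
; Left click toggles selection and tile menus, while E opens the Builder menu.
; Holding right mouse hides the cursor and opens gates that pass mouse movement into yaw and pitch.
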(event EventBeginPlay
  (Variables|/Script/Engine.PlayerController|SetbShowMouseCursor (Game|GetPlayerController 0) true))

(event Collision|EventActorBeginOverlap
  (params (OtherActor :type Actor%20Object%20Reference)))

(event EventTick
  (params (DeltaSeconds :type Float%20%28single-precision%29))
  (bind _returnvalue (Game|GetPlayerController 0))
  (bind (_worldlocation _worlddirection) (Game|Player|ConvertMouseLocationToWorldSpace _returnvalue))
  (Utilities|FlowControl|Sequence
    (:then_0
      (bind _outhit (Collision|LineTraceByChannel _worldlocation (+ (* _worlddirection 4e+03) _worldlocation) "TraceTypeQuery1" false 0 "None"))
      (Utilities|FlowControl|Sequence
        (:then_0
          (bind _astile (Utilities|Casting|CastToTile (Variables|Default|GetHoveredActor)))
          (Rendering|Material|SetVectorParameterValue (Variables|/Game/Blueprints/Tile.Tile_C|GetDynamicMaterial _astile) "Color" "(R=0.811765,G=0.788235,B=0.654902,A=1.000000)" :!class /Script/Engine.MaterialInstanceDynamic))
        (:then_1
          (bind _output_get (Variables|Default|SetHoveredActor (.HitActor (Collision|BreakHitResult _outhit))))
          (bind _astile_2 (Utilities|Casting|CastToTile _output_get))
          (if (== _output_get (Variables|Default|GetSelectedActor))
            (Rendering|Material|SetVectorParameterValue (Variables|/Game/Blueprints/Tile.Tile_C|GetDynamicMaterial _astile_2) "Color" "(R=1.000000,G=0.352941,B=0.000000,A=1.000000)" :!class /Script/Engine.MaterialInstanceDynamic)
            (else
              (Rendering|Material|SetVectorParameterValue (Variables|/Game/Blueprints/Tile.Tile_C|GetDynamicMaterial _astile_2) "Color" "(R=0.200633,G=0.811765,B=0.147978,A=1.000000)" :!class /Script/Engine.MaterialInstanceDynamic))))))
    (:then_1
      (Development|PrintString (Utilities|GetDisplayName (Variables|Default|GetSelectedActor)) true true "(R=1.000000,G=0.000000,B=0.777276,A=1.000000)" DeltaSeconds))
    (:then_2
      (bind _astile_3 (Utilities|Casting|CastToTile (Variables|Default|GetSelectedActor)))
      (Rendering|Material|SetVectorParameterValue (Variables|/Game/Blueprints/Tile.Tile_C|GetDynamicMaterial _astile_3) "Color" "(R=1.000000,G=0.352941,B=0.000000,A=1.000000)" :!class /Script/Engine.MaterialInstanceDynamic))))

(event Input|AxisEvents|InputAxisMoveForward
  (params (AxisValue :type Float%20%28single-precision%29))
  (Transformation|AddActorLocalOffset (Math|Vector|MakeVector (* AxisValue (Variables|Default|GetMoveSpeed)) 0.0 0.0) false false))

(event Input|AxisEvents|InputAxisMoveRight
  (params (AxisValue :type Float%20%28single-precision%29))
  (Transformation|AddActorLocalOffset (Math|Vector|MakeVector 0.0 (* AxisValue (Variables|Default|GetMoveSpeed)) 0.0) false false))

(event Input|MouseEvents|MouseX
  (params (AxisValue :type Float%20%28single-precision%29))
  (Utilities|FlowControl|Gate true
    (:Exit
      (Transformation|AddActorLocalRotation (Math|Rotator|MakeRotator 0.0 0.0 (* AxisValue (Variables|Default|GetRotateSpeed))) false false))))

(event Input|MouseEvents|MouseY
  (params (AxisValue :type Float%20%28single-precision%29))
  (Utilities|FlowControl|Gate true
    (:Exit
      (Transformation|AddLocalRotation (Variables|Default|GetCamera) (Math|Rotator|MakeRotator 0.0 (* AxisValue (Variables|Default|GetRotateSpeed)) 0.0) false false))))

(event Input|MouseEvents|MouseWheelUp
  (params (Key :type Key%20Structure :default "None"))
  (bind _springarm (Variables|Default|GetSpringArm))
  (:Pressed
    (Variables|/Script/Engine.SpringArmComponent|SetTargetArmLength _springarm (- (Variables|/Script/Engine.SpringArmComponent|GetTargetArmLength _springarm) (Variables|Default|GetScrollSpeed)))))

(event Input|MouseEvents|MouseWheelDown
  (params (Key :type Key%20Structure :default "None"))
  (bind _springarm (Variables|Default|GetSpringArm))
  (:Pressed
    (Variables|/Script/Engine.SpringArmComponent|SetTargetArmLength _springarm (+ (Variables|/Script/Engine.SpringArmComponent|GetTargetArmLength _springarm) (Variables|Default|GetScrollSpeed)))))

(event Input|MouseEvents|RightMouseButton
  (params (Key :type Key%20Structure :default "None"))
  (bind _returnvalue (Game|GetPlayerController 0))
  (:Pressed
    (Variables|/Script/Engine.PlayerController|SetbShowMouseCursor _returnvalue false)
    (Utilities|FlowControl|Sequence
      (:then_0
        (Utilities|FlowControl|Gate true) ; enters at Open
      )
      (:then_1
        (Utilities|FlowControl|Gate true) ; enters at Open
      )))
  (:Released
    (Variables|/Script/Engine.PlayerController|SetbShowMouseCursor _returnvalue true)
    (Utilities|FlowControl|Sequence
      (:then_0
        (Utilities|FlowControl|Gate true) ; enters at Close
      )
      (:then_1
        (Utilities|FlowControl|Gate true) ; enters at Close
      ))))

(event Input|MouseEvents|LeftMouseButton
  (params (Key :type Key%20Structure :default "None"))
  (bind _hoveredactor (Variables|Default|GetHoveredActor))
  (:Pressed
    (Utilities|FlowControl|Sequence
      (:then_0
        (bind _astile (Utilities|Casting|CastToTile (Variables|Default|GetSelectedActor)))
        (Rendering|Material|SetVectorParameterValue (Variables|/Game/Blueprints/Tile.Tile_C|GetDynamicMaterial _astile) "Color" "(R=0.811765,G=0.788235,B=0.654902,A=1.000000)" :!class /Script/Engine.MaterialInstanceDynamic))
      (:then_1
        (if (== _hoveredactor (Variables|Default|GetSelectedActor))
          (bind _astile_2 (Utilities|Casting|CastToTile (Variables|Default|GetSelectedActor)))
          (Default|CloseMenu _astile_2)
          (Variables|Default|SetSelectedActor 0)
          (else
            (bind _astile_3 (Utilities|Casting|CastToTile (Variables|Default|GetSelectedActor))
              (:then
                (Default|CloseMenu _astile_3))
              (:CastFailed
                _))
            (bind _output_get (Variables|Default|SetSelectedActor _hoveredactor))
            (bind _astile_4 (Utilities|Casting|CastToTile _output_get))
            (Default|OpenMenu _astile_4)))))))

(event Input|KeyboardEvents|E
  (params (Key :type Key%20Structure :default "None"))
  (:Pressed
    (Default|OpenMenu (Variables|Default|GetBuilder))))

(fn ConstructionScript)