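; BP_ActorSelector handles hovering and selecting actors in the world, notifying them through messages.
; Each Tick it raycasts for the hovered actor, sends hover, unhover and selected-tick messages, and prints the selection's name for debugging.
; SelectActor sends clicked-off and clicked messages, letting the hovered actor decide whether it becomes selected.
; Re-selecting the same actor is meant to deselect it, except BP_WateringCan, which gets Clicked instead.
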(event EventBeginPlay)

(event EventTick
  (params (DeltaSeconds :type Float%20%28single-precision%29))
  (bind _actor (CallFunction|RaycastActor))
  (CallFunction|CheckUnhovered _actor)
  (bind _output_get (Variables|Default|SetHoveredActor _actor))
  (Class|BPIRaycastReceiver|Hovered(Message) _output_get)
  (CallFunction|PrintSelectedActorNameTick DeltaSeconds)
  (Class|BPIRaycastReceiver|SelectedTick(Message) (Variables|Default|GetSelectedActor)))

(fn SelectActor
  (bind _hoveredactor (Variables|Default|GetHoveredActor))
  (Class|BPIRaycastReceiver|ClickedOff(Message) (Variables|Default|GetSelectedActor) (Variables|Default|GetHoveredActor))
  (if (Utilities|IsHoveredActorandSelectedActorEqual)
    (bind _asbp_watering_can (Utilities|Casting|CastToBP_WateringCan (Variables|Default|GetSelectedActor))
      (:then
        (Default|Clicked _asbp_watering_can))
      (:CastFailed
        (Variables|Default|SetSelectedActor 0)))
    (else
      (Class|BPIRaycastReceiver|Clicked(Message) _hoveredactor)
      (bind _success (Class|BPIRaycastReceiver|ShouldSetActor(Message) _hoveredactor))
      (if _success
        (Variables|Default|SetSelectedActor _hoveredactor)))))

(fn PrintSelectedActorNameTick
  (params (dt :type Float%20%28single-precision%29))
  (Development|PrintString (Utilities|GetDisplayName (Variables|Default|GetSelectedActor)) true true "(R=1.000000,G=0.000000,B=0.777276,A=1.000000)" dt))

(fn CheckUnhovered
  (params (Actor :type Actor%20Object%20Reference))
  (bind _hoveredactor (Variables|Default|GetHoveredActor))
  (if (!= Actor _hoveredactor)
    (Class|BPIRaycastReceiver|Unhovered(Message) _hoveredactor)))