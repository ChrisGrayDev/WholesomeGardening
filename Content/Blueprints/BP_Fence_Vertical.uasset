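; Vertical fence piece on the tile grid that automatically connects to neighboring vertical fences with horizontal fence pieces.
; On BeginPlay it finds BP_TileManager, caches its four adjacent tiles and spawns a rotated BP_Fence_Horizontal midway to each one occupied by another vertical fence.
; Both vertical fences register each horizontal piece, so destroying either one removes the connections attached to it.
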(event EventBeginPlay
  (bind _returnvalue (Actor|GetActorOfClass "/Game/Blueprints/BP_TileManager.BP_TileManager_C"))
  (bind _gridposition (Default|ActorLocationtoGridPosition _returnvalue (Transformation|GetActorLocation)))
  (CallFunction|GetAdjacentTiles _gridposition _returnvalue)
  (Variables|Default|SetTileManager _returnvalue)
  (CallFunction|UpdateAdjacentFences))

(event Collision|EventActorBeginOverlap
  (params (OtherActor :type Actor%20Object%20Reference)))

(event EventTick
  (params (DeltaSeconds :type Float%20%28single-precision%29)))

(event EventDestroyed
  (CallFunction|DestroyAllHorizontalFences))

(fn ConstructionScript)

(fn GetAdjacentTiles
  (params (GridPosition :type Vector) (TileManager :type BP%20Tile%20Manager%20Object%20Reference))
  (Utilities|FlowControl|Sequence
    (:then_0
      (bind _tile (Default|GetTilefromGridPosition TileManager (+ (LocalVariables|GetUp) GridPosition)))
      (Utilities|Array|Add (Variables|Default|GetAdjacentTiles) _tile))
    (:then_1
      (bind _tile_2 (Default|GetTilefromGridPosition TileManager (+ GridPosition (LocalVariables|GetDown))))
      (Utilities|Array|Add (Variables|Default|GetAdjacentTiles) _tile_2))
    (:then_2
      (bind _tile_3 (Default|GetTilefromGridPosition TileManager (+ GridPosition (LocalVariables|GetLeft))))
      (Utilities|Array|Add (Variables|Default|GetAdjacentTiles) _tile_3))
    (:then_3
      (bind _tile_4 (Default|GetTilefromGridPosition TileManager (+ GridPosition (LocalVariables|GetRight))))
      (Utilities|Array|Add (Variables|Default|GetAdjacentTiles) _tile_4))))

(fn TileHasFence
  (params (Tile :type BP%20Tile%20Object%20Reference))
  (if (Variables|/Game/Blueprints/BP_Tile.BP_Tile_C|GetIsOccupied Tile)
    (bind _asbp_fence_vertical (Utilities|Casting|CastToBP_Fence_Vertical (Variables|/Game/Blueprints/BP_Tile.BP_Tile_C|GetOccupiedObj Tile))
      (:then
        (return true _asbp_fence_vertical))
      (:CastFailed
        _)))
  (return false 0))

(fn UpdateAdjacentFences
  (for _array_element (Variables|Default|GetAdjacentTiles)
    (CallFunction|UpdateFence _array_element)))

(fn UpdateFence
  (params (Tile :type BP%20Tile%20Object%20Reference))
  (bind _returnvalue (Transformation|GetActorLocation))
  (bind _tilemanager (Variables|Default|GetTileManager))
  (bind (_hasfence _fence) (CallFunction|TileHasFence Tile))
  (if _hasfence
    (bind _gridposition (Default|ActorLocationtoGridPosition _tilemanager _returnvalue))
    (bind _transform (Default|GridPositiontoTransform _tilemanager (- (Variables|/Game/Blueprints/BP_Tile.BP_Tile_C|GetGridPosition Tile) _gridposition)))
    (bind _returnvalue_2 (Game|SpawnActorfromClass "/Game/Blueprints/BP_Fence_Horizontal.BP_Fence_Horizontal_C" (Math|Transform|MakeTransform (+ (+ (* (.location _transform) 0.5) _returnvalue) (Math|Vector|MakeVector (.y (* (- (Variables|/Game/Blueprints/BP_Tile.BP_Tile_C|GetGridPosition Tile) _gridposition) 0.0)) (.x (* (- (Variables|/Game/Blueprints/BP_Tile.BP_Tile_C|GetGridPosition Tile) _gridposition) 0.0)) 0.0)) (Math|Rotator|MakeRotator 0.0 0.0 (* 90 (.X (Math|Vector|BreakVector (- (Variables|/Game/Blueprints/BP_Tile.BP_Tile_C|GetGridPosition Tile) _gridposition))))) "1,1,1") "Undefined" 0 0))
    (CallFunction|AddHorizontalFence _fence _returnvalue_2)
    (CallFunction|AddHorizontalFence _returnvalue_2)))

(fn AddHorizontalFence
  (params (Fence :type BP%20Fence%20Horizontal%20Object%20Reference))
  (Utilities|Array|Add (Variables|Default|GetHorizontalFences) Fence))

(fn DestroyAllHorizontalFences
  (bind _horizontalfences (Variables|Default|GetHorizontalFences))
  (for _array_element _horizontalfences
    (Utilities|IsValid _array_element
      (:Is%20Valid
        (Actor|DestroyActor _array_element))))
  (Utilities|Array|Clear _horizontalfences))