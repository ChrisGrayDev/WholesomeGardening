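; Mouse-driven selector for farming Tiles and watering cans that highlights hovered and selected actors.
; Each Tick traces from the cursor, tints hovered tiles and cans green and the selected tile red through material parameters, and prints the selection name.
; ManageSelection toggles selection and opens or closes tile menus.
; With a can selected, it passes the hovered tile's plant to WateringMechanic, then clears selection, as does picking empty space.
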(event EventBeginPlay)

(event EventTick
  (params (DeltaSeconds :type Float%20%28single-precision%29))
  (Utilities|FlowControl|Sequence
    (:then_0
      (CallFunction|ResetTileColor)
      (bind _actorout (CallFunction|RaycastActor))
      (Utilities|FlowControl|Sequence
        (:then_0
          (if (Utilities|IsClassOfType _actorout "/Game/Blueprints/Tile.Tile_C")
            (CallFunction|UpdateTileColor)))
        (:then_1
          (if (Utilities|IsClassOfType _actorout "/Game/Blueprints/BP_WateringCan.BP_WateringCan_C")
            (bind _asbp_watering_can (Utilities|Casting|CastToBP_WateringCan _actorout))
            (CallFunction|HoverSkeletalObj (Variables|/Game/Blueprints/BP_WateringCan.BP_WateringCan_C|GetSkeletalMesh _asbp_watering_can) true)))
        (:then_2
          (CallFunction|SetSelectedTileColorRed))))
    (:then_1
      (CallFunction|PrintSelectedActorNameTick DeltaSeconds))))

(fn SelectActor
  (bind _hoveredactor (Variables|Default|GetHoveredActor))
  (Utilities|FlowControl|Sequence
    (:then_1
      (CallFunction|SetSelectedTileColorBlank))
    (:then_2
      (if (== _hoveredactor (Variables|Default|GetSelectedActor))
        (bind _astile (Utilities|Casting|CastToTile (Variables|Default|GetSelectedActor)))
        (Default|CloseMenu _astile)
        (Variables|Default|SetSelectedActor 0)
        (else
          (bind _astile_2 (Utilities|Casting|CastToTile (Variables|Default|GetSelectedActor))
            (:then
              (Default|CloseMenu _astile_2))
            (:CastFailed
              _))
          (bind _output_get (Variables|Default|SetSelectedActor _hoveredactor))
          (bind _astile_3 (Utilities|Casting|CastToTile _output_get)
            (:then
              (Default|OpenMenu _astile_3))
            (:CastFailed
              (CallFunction|DeselectObjectNothingSelected))))))))

(fn SetTileColor
  (params (Actor :type Actor%20Object%20Reference) (HoverColor :type Boolean) (Color :type Vector))
  (bind _astile (Utilities|Casting|CastToTile Actor))
  (Rendering|Material|SetScalarParameterValueonMaterials (Variables|/Script/Engine.StaticMeshActor|GetStaticMeshComponent _astile) "IsHovered" (Math|Conversions|ToFloat(Boolean) HoverColor))
  (Rendering|Material|SetVectorParameterValueonMaterials (Variables|/Script/Engine.StaticMeshActor|GetStaticMeshComponent _astile) "HoverColor" Color))

(fn RaycastActor
  (bind _returnvalue (Game|GetPlayerController 0))
  (bind (_worldlocation _worlddirection) (Game|Player|ConvertMouseLocationToWorldSpace _returnvalue))
  (bind _outhit (Collision|LineTraceByChannel _worldlocation (+ (* _worlddirection 5e+03) _worldlocation) "TraceTypeQuery1" true 0 "None"))
  (bind _output_get (Variables|Default|SetHoveredActor (.HitActor (Collision|BreakHitResult _outhit))))
  (return _output_get))

(fn ResetTileColor
  (bind _hoveredactor (Variables|Default|GetHoveredActor))
  (Utilities|Casting|CastToTile _hoveredactor)
  (CallFunction|SetTileColor _hoveredactor false "0, 0, 0"))

(fn UpdateTileColor
  (Utilities|FlowControl|Sequence
    (:then_0
      (CallFunction|SetTileColor (Variables|Default|GetHoveredActor) true "0.230828,0.739583,0.247832"))
    (:then_1
      (CallFunction|SetSelectedTileColorRed))))

(fn PrintSelectedActorNameTick
  (params (dt :type Float%20%28single-precision%29))
  (Development|PrintString (Utilities|GetDisplayName (Variables|Default|GetSelectedActor)) true true "(R=1.000000,G=0.000000,B=0.777276,A=1.000000)" dt))

(fn SetSelectedTileColorRed
  (bind _astile (Utilities|Casting|CastToTile (Variables|Default|GetSelectedActor)))
  (CallFunction|SetTileColor _astile true "0.741176,0.074510,0.074510"))

(fn ManageSelection
  (Utilities|FlowControl|Sequence
    (:then_0
      (if (or (not (Utilities|IsValid (Variables|Default|GetSelectedActor))) (Utilities|IsClassOfType (Variables|Default|GetSelectedActor) "/Game/Blueprints/Tile.Tile_C"))
        (CallFunction|SelectActor)))
    (:then_1
      (if (and (Utilities|IsClassOfType (Variables|Default|GetSelectedActor) "/Game/Blueprints/BP_WateringCan.BP_WateringCan_C") (Utilities|IsClassOfType (Variables|Default|GetHoveredActor) "/Game/Blueprints/Tile.Tile_C"))
        (CallFunction|WaterTile)
        (Variables|Default|SetSelectedActor 0)))
    (:then_2
      (if (and (Utilities|IsClassOfType (Variables|Default|GetSelectedActor) "/Game/Blueprints/BP_WateringCan.BP_WateringCan_C") (not (Utilities|IsValid (Variables|Default|GetHoveredActor))))
        (Variables|Default|SetSelectedActor 0)))))

(fn WaterTile
  (bind _astile (Utilities|Casting|CastToTile (Variables|Default|GetHoveredActor)))
  (bind _asbp_plant (Utilities|Casting|CastToBP_Plant (Variables|/Game/Blueprints/Tile.Tile_C|GetOccupiedObj _astile)))
  (bind _asbp_watering_can (Utilities|Casting|CastToBP_WateringCan (Variables|Default|GetSelectedActor)))
  (Default|WaterPlant (Variables|Default|GetWateringMechanic) _asbp_watering_can _asbp_plant))

(fn SetSelectedTileColorBlank
  (CallFunction|SetTileColor (Variables|Default|GetSelectedActor) false "0, 0, 0"))

(fn DeselectObjectNothingSelected
  (Utilities|IsValid (Variables|Default|GetHoveredActor)
    (:Is%20Not%20Valid
      (CallFunction|SetSelectedTileColorBlank)
      (Variables|Default|SetSelectedActor 0))))