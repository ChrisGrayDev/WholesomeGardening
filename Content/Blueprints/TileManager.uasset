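; TileManager builds a square grid of Tile actors when play begins.
; CreateLocations computes row-major, cell-centered world positions from GridSize and TileSize, using StartingLocation only for height.
; CreateTiles spawns a Tile at each point, stores it by index in Tiles, and sets its Position by subtracting an offset from the location and dividing by TileSize.
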(event EventBeginPlay
  (CallFunction|CreateTiles))

(event Collision|EventActorBeginOverlap
  (params (OtherActor :type Actor%20Object%20Reference)))

(event EventTick
  (params (DeltaSeconds :type Float%20%28single-precision%29)))

(fn ConstructionScript)

(fn CreateTiles
  (bind _gridsize (Variables|Default|GetGridSize))
  (bind _tilesize (Variables|Default|GetTileSize))
  (bind _positions (CallFunction|CreateLocations _gridsize _tilesize))
  (for (_array_element _array_index) _positions
    (bind _returnvalue (Game|SpawnActorfromClass "/Game/Blueprints/Tile.Tile_C" (Math|Conversions|ToTransform(Vector) _array_element) "Undefined" self 0))
    (Utilities|Array|SetArrayElem (Variables|Default|GetTiles) _array_index _returnvalue)
    (bind _position (CallFunction|GetPositionfromLocation _gridsize _tilesize _array_element (.location (Variables|Default|GetStartingLocation))))
    (Variables|/Game/Blueprints/Tile.Tile_C|SetPosition _returnvalue _position)))

(fn CreateLocations
  (params (GridSize :type Integer) (TileSize :type Integer))
  (bind _returnvalue (/ TileSize 2))
  (bind _returnvalue_2 (- GridSize 1))
  (for _index (range 0 _returnvalue_2)
    (for _index_2 (range 0 _returnvalue_2)
      (bind _output_get (Variables|Default|SetCurrentX (+ (* _index_2 TileSize) _returnvalue)))
      (bind _output_get_2 (Variables|Default|SetCurrentY (+ (* _index TileSize) _returnvalue)))
      (bind _output_get_3 (Variables|Default|SetCurrentLocataion (Math|Vector|MakeVector (Math|Conversions|ToFloat(Integer) _output_get) (Math|Conversions|ToFloat(Integer) _output_get_2) (.z (.location (Variables|Default|GetStartingLocation))))))
      (Utilities|Array|SetArrayElem (Variables|Default|GetPositions) (+ _index_2 (* _index GridSize)) _output_get_3 true)))
  (return (Variables|Default|GetPositions)))

(fn GetPositionfromLocation
  (params (GridSize :type Integer) (TileSize :type Integer) (CurrentLocation :type Vector) (OffsetLocation :type Vector))
  (return (/ (- CurrentLocation (LocalVariables|GetOffset)) TileSize)))