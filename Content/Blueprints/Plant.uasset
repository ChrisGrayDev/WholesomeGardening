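; Plant Blueprint that tracks growth time and marks itself as grown after a required duration.
; The Construction Script sets a timer by function name to call GrowPlant, which prints a message and sets HasGrown.
; Tick separately accumulates and prints elapsed time while growth is enabled and unfinished, but that counter does not drive the timer.
; A helper function resets the counter to zero without touching the timer.
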(event EventBeginPlay)

(event Collision|EventActorBeginOverlap
  (params (OtherActor :type Actor%20Object%20Reference)))

(event EventTick
  (params (DeltaSeconds :type Float%20%28single-precision%29))
  (if (and (not (Variables|Default|GetHasGrown)) (Variables|Default|GetEnabledGrowth))
    (bind _output_get (Variables|Default|SetCurrentGrowthTime (+ DeltaSeconds (Variables|Default|GetCurrentGrowthTime))))
    (Development|PrintString (Utilities|String|ToString(Float) _output_get) true true "(R=0.000000,G=0.660000,B=1.000000,A=1.000000)" DeltaSeconds)))

(fn ConstructionScript
  (Utilities|Time|SetTimerbyFunctionName 0 "GrowPlant" (Variables|Default|GetRequiredGrowthTime)))

(fn GrowPlant
  (Development|PrintString "Plant has grown!")
  (Variables|Default|SetHasGrown true))

(fn ResetCurrentGrowthTime
  (Variables|Default|SetCurrentGrowthTime 0.0))