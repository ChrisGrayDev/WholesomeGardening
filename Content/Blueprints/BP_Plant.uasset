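; BP_Plant is a plant actor that handles the visual feedback for smoke bursts and timed processes.
; On BeginPlay it binds handlers to smoke burst and timer spawn events, playing the smoke effect or calling TimerSpawn.
; TimerSpawn spawns a BP_ProgressBar at an offset from the actor and starts it with the given duration.
; The construction script gives the static mesh a dynamic material instance.
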(event Custom|SmokeEvent
  (CallFunction|PlaySmokeBurst (Variables|Default|GetSmoke)))

(event Custom|SpawnTimer
  (params (TimeToFinish :type Float%20%28single-precision%29))
  (CallFunction|TimerSpawn TimeToFinish))

(event EventBeginPlay
  (EventDispatchers|AssignOnSmokeBurst (delegate Custom|SmokeEvent))
  (EventDispatchers|BindEventtoOnTimerSpawn (delegate Custom|SpawnTimer)))

(event Collision|EventActorBeginOverlap
  (params (OtherActor :type Actor%20Object%20Reference)))

(event EventTick
  (params (DeltaSeconds :type Float%20%28single-precision%29)))

(fn ConstructionScript
  (bind _returnvalue (Rendering|Material|CreateDynamicMaterialInstance (Variables|Default|Getst_mesh) 0 0 "None" :!class /Script/Engine.PrimitiveComponent))
  (Rendering|Material|SetMaterial (Variables|Default|Getst_mesh) 0 _returnvalue))

(fn TimerSpawn
  (params (Time :type Float%20%28single-precision%29))
  (bind _returnvalue (Game|SpawnActorfromClass "/Game/Blueprints/BP_ProgressBar.BP_ProgressBar_C" (Math|Transform|MakeTransform (+ (Transformation|GetActorLocation) (Variables|Default|GetTimerOffset))) "Undefined" 0 0))
  (Default|StartTimer _returnvalue Time))