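; TileSelector highlights the Tile under the mouse cursor and manages which Tile is selected.
; Each Tick it resets the previous hover, line traces from the deprojected cursor, tints the hit Tile green and keeps the selected one orange through dynamic material colors.
; SelectTile makes the hovered actor the selection or clears it if already selected, opening and closing Tile menus.
; Tick also prints the selected actor's name on screen.
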(event EventBeginPlay)

(event EventTick
  (params (DeltaSeconds :type Float%20%28single-precision%29))
  (bind _returnvalue (Game|GetPlayerController 0))
  (bind (_worldlocation _worlddirection) (Game|Player|ConvertMouseLocationToWorldSpace _returnvalue))
  (Utilities|FlowControl|Sequence
    (:then_0
      (bind _outhit (Collision|LineTraceByChannel _worldlocation (+ (* _worlddirection 1e+04) _worldlocation) "TraceTypeQuery1" false 0 "None"))
      (Utilities|FlowControl|Sequence
        (:then_0
          (bind _astile (Utilities|Casting|CastToTile (Variables|Default|GetHoveredActor)))
          (Rendering|Material|SetVectorParameterValue (Variables|/Game/Blueprints/Tile.Tile_C|GetDynamicMaterial _astile) "Color" "(R=0.811765,G=0.788235,B=0.654902,A=1.000000)" :!class /Script/Engine.MaterialInstanceDynamic))
        (:then_1
          (bind _output_get (Variables|Default|SetHoveredActor (.HitActor (Collision|BreakHitResult _outhit))))
          (bind _astile_2 (Utilities|Casting|CastToTile _output_get))
          (if (== _output_get (Variables|Default|GetSelectedActor))
            (Rendering|Material|SetVectorParameterValue (Variables|/Game/Blueprints/Tile.Tile_C|GetDynamicMaterial _astile_2) "Color" "(R=1.000000,G=0.352941,B=0.000000,A=1.000000)" :!class /Script/Engine.MaterialInstanceDynamic)
            (else
              (Rendering|Material|SetVectorParameterValue (Variables|/Game/Blueprints/Tile.Tile_C|GetDynamicMaterial _astile_2) "Color" "(R=0.200633,G=0.811765,B=0.147978,A=1.000000)" :!class /Script/Engine.MaterialInstanceDynamic))))))
    (:then_1
      (Development|PrintString (Utilities|GetDisplayName (Variables|Default|GetSelectedActor)) true true "(R=1.000000,G=0.000000,B=0.777276,A=1.000000)" DeltaSeconds))
    (:then_2
      (bind _astile_3 (Utilities|Casting|CastToTile (Variables|Default|GetSelectedActor)))
      (Rendering|Material|SetVectorParameterValue (Variables|/Game/Blueprints/Tile.Tile_C|GetDynamicMaterial _astile_3) "Color" "(R=1.000000,G=0.352941,B=0.000000,A=1.000000)" :!class /Script/Engine.MaterialInstanceDynamic))))

(fn SelectTile
  (bind _hoveredactor (Variables|Default|GetHoveredActor))
  (Utilities|FlowControl|Sequence
    (:then_0
      (bind _astile (Utilities|Casting|CastToTile (Variables|Default|GetSelectedActor)))
      (Rendering|Material|SetVectorParameterValue (Variables|/Game/Blueprints/Tile.Tile_C|GetDynamicMaterial _astile) "Color" "(R=0.811765,G=0.788235,B=0.654902,A=1.000000)" :!class /Script/Engine.MaterialInstanceDynamic))
    (:then_1
      (if (== _hoveredactor (Variables|Default|GetSelectedActor))
        (bind _astile_2 (Utilities|Casting|CastToTile (Variables|Default|GetSelectedActor)))
        (Default|CloseMenu _astile_2)
        (Variables|Default|SetSelectedActor 0)
        (else
          (bind _astile_3 (Utilities|Casting|CastToTile (Variables|Default|GetSelectedActor))
            (:then
              (Default|CloseMenu _astile_3))
            (:CastFailed
              _))
          (bind _output_get (Variables|Default|SetSelectedActor _hoveredactor))
          (bind _astile_4 (Utilities|Casting|CastToTile _output_get))
          (Default|OpenMenu _astile_4))))))