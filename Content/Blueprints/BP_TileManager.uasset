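; BP_TileManager is a manager Blueprint that builds a flat rectangular grid of BP_Tile actors when play begins.
; CreateGrid loops over YLength rows and XLength columns, and SpawnTile places each tile at its grid position scaled by TileSize and offset from StartingLocation.
; Each tile stores its GridPosition and joins the row-major Tiles array, with GridPositionToArrayIndex converting range-checked coordinates into an array index.
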(event EventBeginPlay
  (CallFunction|CreateGrid))

(event Collision|EventActorBeginOverlap
  (params (OtherActor :type Actor%20Object%20Reference)))

(event EventTick
  (params (DeltaSeconds :type Float%20%28single-precision%29)))

(fn ConstructionScript)

(fn CreateGrid
  (for _index (range 0 (- (Variables|Default|GetYLength) 1))
    (for _index_2 (range 0 (- (Variables|Default|GetXLength) 1))
      (CallFunction|SpawnTile (Math|Vector|MakeVector (Math|Conversions|ToFloat(Integer) _index_2) (Math|Conversions|ToFloat(Integer) _index) 0.0)))))

(fn SpawnTile
  (params (GridPosition :type Vector))
  (bind _transform (CallFunction|GridPositiontoTransform GridPosition))
  (bind _returnvalue (Game|SpawnActorfromClass "/Game/Blueprints/BP_Tile.BP_Tile_C" _transform "Undefined" 0 0))
  (Variables|/Game/Blueprints/BP_Tile.BP_Tile_C|SetGridPosition _returnvalue GridPosition)
  (Utilities|Array|Add (Variables|Default|GetTiles) _returnvalue))

(fn GridPositiontoTransform
  (params (GridPosition :type Vector))
  (return (Math|Transform|MakeTransform (+ (* GridPosition (Variables|Default|GetTileSize)) (Variables|Default|GetStartingLocation)) "0, 0, 0" "1,1,1")))

(fn GridPositiontoArrayIndex
  (params (GridPosition :type Vector))
  (if (and (Utilities|IntegerinRange (Math|Float|Truncate (.x GridPosition)) 0 (Variables|Default|GetXLength)) (Utilities|IntegerinRange (Math|Float|Truncate (.y GridPosition)) 0 (Variables|Default|GetYLength)))
    (return (Math|Float|Truncate (+ (.x GridPosition) (* (Variables|Default|GetXLength) (.y GridPosition)))))))