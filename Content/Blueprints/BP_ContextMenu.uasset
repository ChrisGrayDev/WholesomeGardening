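; BP_ContextMenu is an in-world actor that shows a menu of context choices for a given tile.
; Its widget component hosts a WBP_ContextList and rotates every tick to face the player camera.
; PopulateContextMenu converts each available context enum to a row name, looks it up in ContextTable, and passes the gathered rows, tile and itself to the list.
; DestroyMenu removes the actor.
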(event EventBeginPlay
  (bind _aswbp_context_list (Utilities|Casting|CastToWBP_ContextList (UserInterface|GetWidget (Variables|Default|GetWidget))))
  (Variables|Default|SetContextWidget _aswbp_context_list))

(event Collision|EventActorBeginOverlap
  (params (OtherActor :type Actor%20Object%20Reference)))

(event EventTick
  (params (DeltaSeconds :type Float%20%28single-precision%29))
  (bind _widget (Variables|Default|GetWidget))
  (Transformation|SetWorldRotation _widget (Math|Rotator|FindLookatRotation (Transformation|GetWorldLocation _widget) (Transformation|GetActorLocation (Game|GetPlayerCameraManager 0))) false false))

(fn ConstructionScript)

(fn PopulateContextMenu
  (params (AvailableContexts :type Array%20of%20ContextSelect%20Enums :default "NewEnumerator0") (TileIn :type BP%20Tile%20Object%20Reference))
  (bind _contextbuttonchoices (LocalVariables|GetContextButtonChoices))
  (Variables|Default|SetCurrentTile TileIn)
  (for _array_element AvailableContexts
    (bind _returnvalue (Utilities|GetDataTableRow (Variables|Default|GetContextTable) (Utilities|String|StringToName (Utilities|String|EnumtoString _array_element)))
      (:then
        (Utilities|Array|Add _contextbuttonchoices _returnvalue))))
  (Default|PopulateList (Variables|Default|GetContextWidget) _contextbuttonchoices (Variables|Default|GetCurrentTile) self))

(fn DestroyMenu
  (Actor|DestroyActor))