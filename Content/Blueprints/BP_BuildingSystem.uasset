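; Tile-based building system that previews and places soil, plants and decorations on BP_Tile actors.
; While building, Tick raycasts for the hovered tile and maintains a snapped preview hologram, rotatable in 90-degree steps and coloured by occupancy.
; Placement rejects occupied tiles, spawns by item type and hands the actor to the tile, with ContinuousBuilding deciding whether build mode persists.
; Soil and plants initialise from data tables; decorations always spawn BP_Fence_Vertical.
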(event EventBeginPlay)

(event EventTick
  (params (DeltaSeconds :type Float%20%28single-precision%29))
  (if (Variables|Default|GetIsBuilding)
    (CallFunction|GetHoveredTile)
    (CallFunction|SpawnHologram)
    (CallFunction|UpdateHologramProperties)
    (CallFunction|SnapHologramtoTile)
    (else
      (CallFunction|DestroyHologram (Variables|Default|GetHologram)))))

(fn PlaceActoronTile
  (bind _hoveredtile (Variables|Default|GetHoveredTile))
  (if (Variables|Default|GetIsBuilding)
    (Utilities|IsValid _hoveredtile
      (:Is%20Valid
        (if (Variables|/Game/Blueprints/BP_Tile.BP_Tile_C|GetIsOccupied _hoveredtile)
          (Development|PrintString "Cannot build here")
          (else
            (bind _item (CallFunction|SpawnItem))
            (Utilities|IsValid _item
              (:Is%20Valid
                (bind _asbp_soil (Utilities|Casting|CastToBP_Soil _item)
                  (:then
                    (bind _successful (Default|AddSoiltoTile (Variables|Default|GetHoveredTile) _asbp_soil))
                    (Variables|Default|SetIsBuilding (not _successful)))
                  (:CastFailed
                    (bind _successful_2 (Default|AddObjecttoTile (Variables|Default|GetHoveredTile) _item (Variables|Default|GetRotationSnapOffset)))
                    (Variables|Default|SetIsBuilding (not _successful_2))))
                (CallFunction|DestroyHologram (Variables|Default|GetHologram))
                (Variables|Default|SetIsBuilding (Variables|Default|GetContinuousBuilding))))))))))

(fn ToggleIsBuilding
  (params (IsBuilding :type Boolean))
  (bind _output_get (Variables|Default|SetIsBuilding IsBuilding))
  (if _output_get
    (CallFunction|ToggleTileVisibility true)
    (CallFunction|DestroyHologram (Variables|Default|GetHologram))
    (else
      (CallFunction|ToggleTileVisibility false))))

(fn RotateOffset
  (params (Clockwise :type Boolean))
  (if Clockwise
    (bind _output_get (Variables|Default|SetRotationSnapOffset (+ (Variables|Default|GetRotationSnapOffset) 90)))
    (else
      (Variables|Default|SetRotationSnapOffset (+ (Variables|Default|GetRotationSnapOffset) -90))))
  (if (>= _output_get 360)
    (Variables|Default|SetRotationSnapOffset (+ (Variables|Default|GetRotationSnapOffset) -360))
    (elif (not (>= (Variables|Default|GetRotationSnapOffset) 0))
      (Variables|Default|SetRotationSnapOffset (+ (Variables|Default|GetRotationSnapOffset) 360)))))

(fn SpawnPlantfromTable
  (params (Item :type Item%20Data%20Structure))
  (bind _returnvalue (Game|SpawnActorfromClass "/Game/Blueprints/BP_Plant.BP_Plant_C" (Variables|Default|GetTilePlaceTransform) "Undefined" 0 0))
  (bind _returnvalue_2 (Utilities|GetDataTableRow (Variables|Default|GetPlantTable) (Utilities|String|StringToName (.name (Utilities|Struct|BreakItemData Item))))
    (:then
      (Class|Plant|InitPlant _returnvalue _returnvalue_2)
      (return _returnvalue))
    (:RowNotFound
      (return _returnvalue))))

(fn SpawnDecorationfromTable
  (params (Item :type Item%20Data%20Structure))
  (bind _returnvalue (Game|SpawnActorfromClass "/Game/Blueprints/BP_Fence_Vertical.BP_Fence_Vertical_C" (Variables|Default|GetTilePlaceTransform) "Undefined" 0 0))
  (return _returnvalue))

(fn GetHoveredTile
  (if (Variables|Default|GetIsBuilding)
    (bind _actor (CallFunction|RaycastActor))
    (bind _asbp_tile (Utilities|Casting|CastToBP_Tile _actor)
      (:then
        (Variables|Default|SetHoveredTile _asbp_tile))
      (:CastFailed
        (Variables|Default|SetHoveredTile 0)
        (CallFunction|DestroyHologram (Variables|Default|GetHologram))))))

(fn SnapHologramtoTile
  (bind _hologram (Variables|Default|GetHologram))
  (Utilities|IsValid _hologram
    (:Is%20Valid
      (Transformation|SetActorLocationAndRotation _hologram (.location (Variables|Default|GetTilePlaceTransform)) (Math|Rotator|MakeRotator 0.0 0.0 (Math|Conversions|ToFloat(Integer) (Variables|Default|GetRotationSnapOffset)))))))

(fn DestroyHologram
  (params (Actor :type Actor%20Object%20Reference))
  (if (Utilities|IsValid Actor)
    (Actor|DestroyActor Actor)
    (Variables|Default|SetTilePlaceTransform "")))

(fn SpawnHologram
  (Utilities|IsValid (Variables|Default|GetHologram)
    (:Is%20Not%20Valid
      (Utilities|IsValid (Variables|Default|GetHoveredTile)
        (:Is%20Valid
          (bind _returnvalue (Utilities|GetDataTableRow "/Game/Data/DT_PlaceableObjData.DT_PlaceableObjData" (Utilities|String|StringToName (.name (Variables|Default|GetActiveItem))))
            (:then
              (bind _returnvalue_2 (Game|SpawnActorfromClass "/Game/Blueprints/BP_PreviewObj.BP_PreviewObj_C" (Variables|Default|GetTilePlaceTransform) "Undefined" 0 0))
              (Default|InitMesh _returnvalue_2 (.mesh _returnvalue))
              (Variables|Default|SetHologram _returnvalue_2))))))))

(fn UpdateHologramProperties
  (bind _hoveredtile (Variables|Default|GetHoveredTile))
  (bind _hologram (Variables|Default|GetHologram))
  (Utilities|IsValid _hoveredtile
    (:Is%20Valid
      (Variables|Default|SetTilePlaceTransform (Transformation|GetActorTransform _hoveredtile))
      (Utilities|IsValid _hologram
        (:Is%20Valid
          (bind _asbp_preview_obj (Utilities|Casting|CastToBP_PreviewObj _hologram))
          (Default|SetHologramColour _asbp_preview_obj (not (Variables|/Game/Blueprints/BP_Tile.BP_Tile_C|GetIsOccupied _hoveredtile))))))))

(fn SpawnItem
  (bind _activeitem (Variables|Default|GetActiveItem))
  (switch Utilities|FlowControl|Switch|SwitchonEItemType (.item_type (Variables|Default|GetActiveItem))
    (:Plant
      (if (Utilities|Enum|Equal(Enum) (.item_category (Utilities|Struct|BreakItemData _activeitem)) "Soil")
        (if (Variables|/Game/Blueprints/BP_Tile.BP_Tile_C|GetHasSoil (Variables|Default|GetHoveredTile))
          _
          (else
            _))
        (bind _out (CallFunction|SpawnSoilfromTable _activeitem))
        (return _out)
        (else
          (bind _out_2 (CallFunction|SpawnPlantfromTable _activeitem))
          (return _out_2))))
    (:Object
      (bind _decoration (CallFunction|SpawnDecorationfromTable _activeitem))
      (return _decoration))))

(fn SpawnSoilfromTable
  (params (Item :type Item%20Data%20Structure))
  (bind _returnvalue (Game|SpawnActorfromClass "/Game/Blueprints/BP_Soil.BP_Soil_C" (Variables|Default|GetTilePlaceTransform) "Undefined" 0 0))
  (bind _returnvalue_2 (Utilities|GetDataTableRow (Variables|Default|GetSoilTable) (Utilities|String|StringToName (.name (Utilities|Struct|BreakItemData Item))))
    (:then
      (Default|SetSoil _returnvalue _returnvalue_2)
      (return _returnvalue))
    (:RowNotFound
      (return _returnvalue))))