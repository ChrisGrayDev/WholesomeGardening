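; Watering Blueprint that lets a watering can water a given plant.
; WaterPlant stores both references, then, if the can is not empty and not both refilling and extracting, teleports it beside the plant, targets it and extracts one charge.
; The event graph runs nothing, holding only unconnected nodes that initialize a plant from a Sunflower data table row and start its growth.
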(event EventBeginPlay)

(event EventTick
  (params (DeltaSeconds :type Float%20%28single-precision%29)))

(fn WaterPlant
  (params (WateringCan :type Watering%20Can%20Object%20Reference) (Plant :type BP%20Plant%20Object%20Reference))
  (Variables|Default|SetWateringCan WateringCan)
  (Variables|Default|SetPlant Plant)
  (bind _returnvalue (Class|WaterExtractable|IsEmpty (Variables|Default|GetWateringCan)))
  (if (not _returnvalue)
    (if (not (and (Variables|/Script/WholesomeGardening.WaterContainer|Getis_refilling (Variables|Default|GetWateringCan)) (Variables|/Script/WholesomeGardening.WaterContainer|Getis_extracting (Variables|Default|GetWateringCan))))
      (Class|WaterExtractable|TeleporttoPoint (Variables|Default|GetWateringCan) (+ (Transformation|GetActorLocation (Variables|Default|GetPlant)) "80.000000,0.000000, 0"))
      (Class|WaterContainer|SetTargetPlant (Variables|Default|GetWateringCan) (Variables|Default|GetPlant))
      (Class|WaterExtractable|ExtractOneCharge (Variables|Default|GetWateringCan)))))